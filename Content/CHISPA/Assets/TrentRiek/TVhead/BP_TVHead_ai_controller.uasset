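; TV Head AI character (despite the controller name) that feeds player detection to a blackboard.
; BeginPlay caches the player and writes the AI type to the blackboard.
; PawnSensing sets the Player key when a visibility trace is clear, then clears it through a retriggerable delay once sightings stop.
; An older Idle/Chase/Attack state machine remains, but its driving switch is disconnected, Tick is empty and attack only prints.
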(event OnSeePawn(PawnSensing)
  (params (Pawn :type Pawn%20Object%20Reference))
  (bind _returnvalue (Pawn|GetController))
  (bind _returnvalue_2 (Utilities|Name|MakeLiteralName "Player"))
  (bind _returnvalue_3 (AI|GetBlackboard _returnvalue))
  ;[1 1 1] look for player
  (Utilities|FlowControl|Sequence
    (:then_0
      (bind _asbp_tvhead_character (Utilities|Casting|CastToBP_TVHead_Character Pawn))
      (bind _isclear (CallFunction|PathCleartoPlayer))
      (if _isclear
        (AI|Components|Blackboard|SetValueasObject _returnvalue_3 _returnvalue_2 _asbp_tvhead_character)))
    (:then_1
      (Utilities|FlowControl|RetriggerableDelay 0.6)
      (AI|Components|Blackboard|SetValueasObject _returnvalue_3 _returnvalue_2 0))))

(event Custom|end%20idle
  ;[1 1 1] Old
  ;;[1 1 1] idle_state
  (Utilities|FlowControl|Gate true) ; enters at Close
)

(event Custom|Chase
  ;[1 1 1] Old
  ;;[1 1 1] Chase
  (AI|Navigation|SimpleMovetoActor (AI|GetAIController self) (Variables|Default|GetplayerR)))

(event Custom|idle
  (bind _returnvalue (Transformation|GetActorLocation))
  (bind _randomlocation (AI|Navigation|GetRandomReachablePointinRadius _returnvalue 5e+03 0 0))
  ;[1 1 1] Old
  ;;[1 1 1] idle
  (Utilities|FlowControl|DoOnce false
    (:Completed
      (AI|AIMoveTo self _randomlocation 0 5.0 false
        (:then
          (Development|PrintString (Utilities|String|ToString(Vector) _randomlocation) true true "(R=0.000000,G=0.660000,B=1.000000,A=1.000000)" 1e+01))
        (:OnSuccess
          (Utilities|FlowControl|Delay (Math|Random|RandomFloatinRange 3.0 1e+01))
          (CallFunction|Resetidle))))))

(event Custom|resetidle
  (bind _returnvalue (Transformation|GetActorLocation))
  (bind _randomlocation (AI|Navigation|GetRandomReachablePointinRadius _returnvalue 5e+03 0 0))
  ;[1 1 1] Old
  ;;[1 1 1] idle
  (Utilities|FlowControl|DoOnce false) ; enters at Reset
)

(event Custom|resetattack
  ;[1 1 1] Old
  ;;[1 1 1] attack
  (Utilities|FlowControl|DoOnce false) ; enters at Reset
)

(event Custom|attack
  ;[1 1 1] Old
  ;;[1 1 1] attack
  (Utilities|FlowControl|DoOnce false
    (:Completed
      (Development|PrintString "Ouch!")
      (Utilities|FlowControl|Delay (Variables|Default|Getattack_rate%28secs%29)))))

(event EventBeginPlay
  ;[1 1 1] set player reference
  (bind _asbp_tvhead_character (Utilities|Casting|CastToBP_TVHead_Character (Game|GetPlayerCharacter 0)))
  (Variables|Default|SetplayerR _asbp_tvhead_character)
  (AI|Components|Blackboard|SetValueasEnum (AI|GetBlackboard (Pawn|GetController)) (Utilities|Name|MakeLiteralName "aiType") (Variables|Default|Getaitype)))

(event EventTick
  (params (DeltaSeconds :type Float%20%28single-precision%29)))

(fn ConstructionScript)

(fn PathCleartoPlayer
  (bind _outhit (Collision|LineTraceByChannel (Transformation|GetActorLocation) (Transformation|GetActorLocation (Variables|Default|GetplayerR)) "TraceTypeQuery1" false 0 "None"))
  (return (not (.bBlockingHit (Collision|BreakHitResult _outhit)))))

(fn ChangeState
  (params (newState :type ai_States%20Enum :default "NewEnumerator0"))
  (Class|NavMovementComponent|StopActiveMovement (Variables|Character|GetCharacterMovement))
  (Variables|Default|SetAi_States newState)
  (CallFunction|Resetidle)
  (CallFunction|Resetattack))

(fn Getdistancetoplayer
  (bind _returnvalue (Transformation|GetActorLocation))
  (bind _playerr (Variables|Default|GetplayerR))
  (bind _returnvalue_2 (Transformation|GetActorLocation _playerr))
  (bind _returnvalue_3 (- _returnvalue_2 _returnvalue))
  (return (Math|Float|Sqrt (+ (Math|Float|Square (.x _returnvalue_3)) (Math|Float|Square (.y _returnvalue_3)) (Math|Float|Square (.z _returnvalue_3))))))